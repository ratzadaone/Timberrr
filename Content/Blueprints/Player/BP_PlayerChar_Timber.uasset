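; Paper2D player character for the Timber game, with four-way movement, a timed main action and speed or axe pickups.
; Movement turns a collision box that highlights overlapped actors; Fire plays a directional flipbook, then messages those actors through interface-style calls.
; Flipbooks and scales come from DT_Flipbooks, keyed by player number, with Tick restoring idle poses.
; FnSpawn only labels the player; its teleport to PlayerStart is disconnected.
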(event OnComponentEndOverlap(CollisionBox)
  (params (OverlappedComponent :type Primitive%20Component%20Object%20Reference) (OtherActor :type Actor%20Object%20Reference) (OtherComp :type Primitive%20Component%20Object%20Reference) (OtherBodyIndex :type Integer))
  (Class|IPlayerInteract|Highlight(Message) OtherActor false))

(event OnComponentBeginOverlap(CollisionBox)
  (params (OverlappedComponent :type Primitive%20Component%20Object%20Reference) (OtherActor :type Actor%20Object%20Reference) (OtherComp :type Primitive%20Component%20Object%20Reference) (OtherBodyIndex :type Integer) (bFromSweep :type Boolean) (SweepResult :type Hit%20Result%20Structure%20%28by%20ref%29))
  (Class|IPlayerInteract|Highlight(Message) OtherActor true))

(event EventBeginPlay
  (Utilities|IsValid (Variables|Default|GetGameModeRef)
    (:Is%20Valid
      _)
    (:Is%20Not%20Valid
      (Variables|Default|SetGameModeRef (.AsBP%20Game%20Mode%20Timber (Utilities|Casting|CastToBP_GameMode_Timber (Game|GetGameMode))))))
  (CallFunction|FnSpawn)
  (bind _flip (CallFunction|FnGetFlipbookfromTable "NewEnumerator8"))
  (Sprite|SetFlipbook (Variables|Default|GetSprite) _flip))

(event EventPickUpPickup
  (params (Pickup :type BP%20Pickup%20Master%20Object%20Reference))
  (bind (_asbp_pickup_speed _bsuccess) (Utilities|Casting|CastToBP_PickupSpeed Pickup))
  (bind _charactermovement (Variables|Character|GetCharacterMovement))
  (if _bsuccess
    (bind _returnvalue (Utilities|Time|SetTimerbyFunctionName 0 "fnSpeedUpEnd" (Variables|/Game/Blueprints/MapActors/Interactive/BP_PickupSpeed.BP_PickupSpeed_C|GetSpedTime _asbp_pickup_speed)))
    (Variables|Default|SetSpeedupTimer _returnvalue)
    (Variables|/Script/Engine.CharacterMovementComponent|SetMaxWalkSpeed _charactermovement (+ (Variables|/Script/Engine.CharacterMovementComponent|GetMaxWalkSpeed _charactermovement) (Variables|/Game/Blueprints/MapActors/Interactive/BP_PickupSpeed.BP_PickupSpeed_C|GetSpeedbost _asbp_pickup_speed)))
    (Actor|DestroyActor _asbp_pickup_speed)
    (elif (.bSuccess (Utilities|Casting|CastToBP_PickupAxe Pickup))
      (Math|Float|IncrementFloat (Variables|Default|GetPower)))))

(event EventTick
  (params (DeltaSeconds :type Float%20%28single-precision%29))
  (if (Math|Boolean|ANDBoolean (== (stale Input|AxisEvents|InputAxisMove_Right AxisValue) 0.0) (== (stale Input|AxisEvents|InputAxisMove_Up AxisValue) 0.0) (Utilities|Enum|NotEqual(Enum) (Variables|Default|GetPlayerFLipState) "NewEnumerator8") (Utilities|Enum|NotEqual(Enum) (Variables|Default|GetPlayerFLipState) "NewEnumerator9") (Utilities|Enum|NotEqual(Enum) (Variables|Default|GetPlayerFLipState) "NewEnumerator10") (Utilities|Enum|NotEqual(Enum) (Variables|Default|GetPlayerFLipState) "NewEnumerator11"))
    (switch Utilities|FlowControl|Switch|SwitchonEnumPlayerFacing (Variables|Default|GetPlayerFacing)
      (:NewEnumerator0
        (CallFunction|FnGetFlipbookfromTable "NewEnumerator10")
        (Variables|Default|SetPlayerFLipState "NewEnumerator10"))
      (:NewEnumerator1
        (CallFunction|FnGetFlipbookfromTable "NewEnumerator11")
        (Variables|Default|SetPlayerFLipState "NewEnumerator11"))
      (:NewEnumerator2
        (CallFunction|FnGetFlipbookfromTable "NewEnumerator9")
        (Variables|Default|SetPlayerFLipState "NewEnumerator9"))
      (:NewEnumerator3
        (CallFunction|FnGetFlipbookfromTable "NewEnumerator8")
        (Variables|Default|SetPlayerFLipState "NewEnumerator8")))))

(event Input|ActionEvents|InputActionFire
  (params (Key :type Key%20Structure :default "AnyKey"))
  (bind _collisionbox (Variables|Default|GetCollisionBox))
  (bind _sprite (Variables|Default|GetSprite))
  (bind _overlappingactors (Collision|GetOverlappingActors _collisionbox 0 :!class /Script/Engine.PrimitiveComponent))
  (bind _returnvalue (Class|PaperFlipbookComponent|GetFlipbookLength _sprite))
  (:Pressed
    (switch Utilities|FlowControl|Switch|SwitchonEnumPlayerFacing (Variables|Default|GetPlayerFacing)
      (:NewEnumerator0
        (CallFunction|FnGetFlipbookfromTable "NewEnumerator7")
        (Utilities|FlowControl|Delay _returnvalue)
        (for _array_element _overlappingactors
          (Class|IPlayerInteract|MainActionBtn(Message) _array_element)
          (CallFunction|FnGetFlipbookfromTable "NewEnumerator10")
          (Variables|Default|SetPlayerFLipState "NewEnumerator10")))
      (:NewEnumerator1
        (CallFunction|FnGetFlipbookfromTable "NewEnumerator7")
        (Utilities|FlowControl|Delay _returnvalue)
        (for _array_element_2 _overlappingactors
          (Class|IPlayerInteract|MainActionBtn(Message) _array_element_2)
          (CallFunction|FnGetFlipbookfromTable "NewEnumerator11")
          (Variables|Default|SetPlayerFLipState "NewEnumerator11")))
      (:NewEnumerator2
        (CallFunction|FnGetFlipbookfromTable "NewEnumerator4")
        (Utilities|FlowControl|Delay _returnvalue)
        (for _array_element_3 _overlappingactors
          (Class|IPlayerInteract|MainActionBtn(Message) _array_element_3)
          (CallFunction|FnGetFlipbookfromTable "NewEnumerator9")
          (Variables|Default|SetPlayerFLipState "NewEnumerator9")))
      (:NewEnumerator3
        (CallFunction|FnGetFlipbookfromTable "NewEnumerator3")
        (Utilities|FlowControl|Delay _returnvalue)
        (for _array_element_4 _overlappingactors
          (Class|IPlayerInteract|MainActionBtn(Message) _array_element_4)
          (CallFunction|FnGetFlipbookfromTable "NewEnumerator8")
          (Variables|Default|SetPlayerFLipState "NewEnumerator8"))))))

(event Input|AxisEvents|InputAxisMove_Right
  (params (AxisValue :type Float%20%28single-precision%29))
  (Pawn|Input|AddMovementInput "0.000000,1.000000, 0" AxisValue false)
  (CallFunction|FnCharTurn (Math|Float|Ceil AxisValue)))

(event Input|AxisEvents|InputAxisMove_Up
  (params (AxisValue :type Float%20%28single-precision%29))
  (if (== (Input|AxisValues|GetMove_Right) 0.0)
    (Pawn|Input|AddMovementInput "1.000000,0.000000, 0" AxisValue false)
    (CallFunction|FnCharTurn 0 (Math|Float|Ceil AxisValue))))

(fn ConstructionScript)

(fn FnCharTurn
  (params (x :type Integer) (y :type Integer))
  (bind _collisionbox (Variables|Default|GetCollisionBox))
  (if (or (!= x 0) (!= y 0))
    (Transformation|SetWorldRotation _collisionbox (Math|Rotator|MakeRotator 0.0 (* y 9e+01) (* x 9e+01)) false false)
    (Transformation|SetRelativeLocation _collisionbox (Math|Vector|MakeVector (* y 2e+01) (* x 2e+01) -5e+01) false false)
    (if (and (> x 0) (Utilities|Enum|NotEqual(Enum) (Variables|Default|GetPlayerFLipState) "NewEnumerator0"))
      (CallFunction|FnGetFlipbookfromTable "NewEnumerator0")
      (Transformation|SetRelativeRotation (Variables|Default|GetSprite) (Math|Rotator|MakeRotator 0.0 0.0 9e+01) false false)
      (Variables|Default|SetPlayerFLipState "NewEnumerator0")
      (Variables|Default|SetPlayerFacing "NewEnumerator1")
      (return)
      (elif (and (< x 0) (Utilities|Enum|NotEqual(Enum) (Variables|Default|GetPlayerFLipState) "NewEnumerator6"))
        (CallFunction|FnGetFlipbookfromTable "NewEnumerator0")
        (Transformation|SetRelativeRotation (Variables|Default|GetSprite) (Math|Rotator|MakeRotator 0.0 0.0 -9e+01) false false)
        (Variables|Default|SetPlayerFLipState "NewEnumerator6")
        (Variables|Default|SetPlayerFacing "NewEnumerator0")
        (return)
        (elif (and (> y 0) (Utilities|Enum|NotEqual(Enum) (Variables|Default|GetPlayerFLipState) "NewEnumerator1"))
          (CallFunction|FnGetFlipbookfromTable "NewEnumerator1")
          (Variables|Default|SetPlayerFLipState "NewEnumerator1")
          (Variables|Default|SetPlayerFacing "NewEnumerator2")
          (return)
          (elif (and (< y 0) (Utilities|Enum|NotEqual(Enum) (Variables|Default|GetPlayerFLipState) "NewEnumerator5"))
            (CallFunction|FnGetFlipbookfromTable "NewEnumerator5")
            (Variables|Default|SetPlayerFLipState "NewEnumerator5")
            (Variables|Default|SetPlayerFacing "NewEnumerator3")
            (return)
            (else
              (return))))))))

(fn FnSpawn
  (bind _playerint (Variables|Default|GetPlayerInt))
  (bind _returnvalue (Utilities|String|ToString(Integer) _playerint))
  (bind _returnvalue_2 (Utilities|String|Append "Player" _returnvalue))
  (bind _outactors (Actor|GetAllActorsOfClass "/Script/Engine.PlayerStart"))
  (for _array_element _outactors
    (if (Utilities|Name|Equal(Name) (Variables|/Script/Engine.PlayerStart|GetPlayerStartTag _array_element) (Utilities|String|StringToName _returnvalue_2))
      (Rendering|Components|TextRender|SetText (Variables|Default|GetTextRender) (Utilities|Text|ToText(String) _returnvalue_2)))))

(fn FnGetFlipbookfromTable
  (params (Flipbook_type_In :type Enum_FlipbooksTypes%20Enum))
  (bind _sprite (Variables|Default|GetSprite))
  (bind _returnvalue (Utilities|GetDataTableRow "/Game/Blueprints/Data/DT_Flipbooks.DT_Flipbooks" (Utilities|String|StringToName (Utilities|String|Append "Player" (Utilities|String|ToString(Integer) (Variables|Default|GetPlayerInt)))))
    (:then
      (Sprite|SetFlipbook _sprite (.Flipbook (Utilities|Struct|BreakStruct_FlipSize (.Value (Utilities|Map|Find (Utilities|Struct|BreakStruct_Flipbook_Properies (.Flipbooks (Utilities|Struct|BreakStruct_Flipbooks _returnvalue))) Flipbook_type_In)))))
      (Transformation|SetRelativeScale3D _sprite (Math|Vector|MakeVector (.X (Math|Vector2D|BreakVector2D (.Scale (Utilities|Struct|BreakStruct_FlipSize (.Value (Utilities|Map|Find (Utilities|Struct|BreakStruct_Flipbook_Properies (.Flipbooks (Utilities|Struct|BreakStruct_Flipbooks _returnvalue))) Flipbook_type_In)))))) 0.25 (.Y (Math|Vector2D|BreakVector2D (.Scale (Utilities|Struct|BreakStruct_FlipSize (.Value (Utilities|Map|Find (Utilities|Struct|BreakStruct_Flipbook_Properies (.Flipbooks (Utilities|Struct|BreakStruct_Flipbooks _returnvalue))) Flipbook_type_In))))))))
      (return (.Flipbook (Utilities|Struct|BreakStruct_FlipSize (.Value (Utilities|Map|Find (Utilities|Struct|BreakStruct_Flipbook_Properies (.Flipbooks (Utilities|Struct|BreakStruct_Flipbooks _returnvalue))) Flipbook_type_In))))))))

(fn FnSpeedUpEnd
  (Variables|/Script/Engine.CharacterMovementComponent|SetMaxWalkSpeed (Variables|Character|GetCharacterMovement) 6e+02)
  (Utilities|Time|ClearandInvalidateTimerbyHandle (Variables|Default|GetSpeedupTimer))
  (Development|PrintString "END"))