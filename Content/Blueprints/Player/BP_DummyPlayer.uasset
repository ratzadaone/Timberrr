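; BP_DummyPlayer is a placeholder pawn that turns into a playable character when Fire is pressed, apparently for local player join.
; It reads its controller ID, calls CreatePlayer, then spawns a BP_PlayerChar_Timber high above the world origin with that ID as PlayerInt.
; The matching player controller possesses the new character, which is registered in the Timber game mode's PlayersInGame list before the dummy destroys itself.
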(event EventBeginPlay
  (Utilities|IsValid (Variables|Default|GetGameModeRef)
    (:Is%20Valid)
    (:Is%20Not%20Valid
      (Variables|Default|SetGameModeRef (.AsBP%20Game%20Mode%20Timber (Utilities|Casting|CastToBP_GameMode_Timber (Game|GetGameMode)))))))

(event Input|ActionEvents|InputActionFire
  (params (Key :type Key%20Structure :default "AnyKey"))
  (:Pressed
    (bind _returnvalue (Class|GameplayStatics|GetPlayerControllerID (.AsBP%20Player%20Controller%20Timber (Utilities|Casting|CastToBP_PlayerController_Timber (Pawn|GetController self)))))
    (Class|GameplayStatics|CreatePlayer _returnvalue)
    (bind _returnvalue_2 (Game|SpawnActorfromClass "/Game/Blueprints/Player/BP_PlayerChar_Timber.BP_PlayerChar_Timber_C" (Math|Transform|MakeTransform "0, 0,2000.000000") "Undefined" 0 _returnvalue 0))
    (Pawn|Possess (Game|GetPlayerController _returnvalue) _returnvalue_2)
    (Utilities|Array|AddUnique (Variables|/Game/Blueprints/Game/BP_GameMode_Timber.BP_GameMode_Timber_C|GetPlayersInGame (Variables|Default|GetGameModeRef)) _returnvalue_2)
    (Actor|DestroyActor)))

(fn ConstructionScript)